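; BP_TreeGen is a tree Blueprint that builds a randomized tree from interchangeable trunk and leaf meshes.
; Its construction script picks a random entry from the Trunkmesh and Leavesmesh arrays and assigns them to the RandomTrunk and RandomLeaves mesh components.
; The picks use unseeded random integers, so the look can change whenever construction reruns, and the event graph has no active logic.
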(fn `UserConstructionScript`
  (bind _leavesmesh (`self.Leavesmesh`))
  (bind _trunkmesh (`self.Trunkmesh`))
  (`StaticMeshComponent.SetStaticMesh` (`self.RandomTrunk`) (`|GetArrayItem` _trunkmesh (`KismetMathLibrary.RandomIntegerInRange` 0 (- (`KismetArrayLibrary.Array_Length` _trunkmesh) 1))))
  (`StaticMeshComponent.SetStaticMesh` (`self.RandomLeaves`) (`|GetArrayItem` _leavesmesh (`KismetMathLibrary.RandomIntegerInRange` 0 (- (`KismetArrayLibrary.Array_Length` _leavesmesh) 1)))))